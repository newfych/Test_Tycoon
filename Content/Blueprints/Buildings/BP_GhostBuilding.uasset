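; Placement preview actor for build mode, showing the selected building's mesh snapped to a grid at the cursor's world position.
; ConstructBuilding briefly spawns the building class to read its mesh and construction proxy, restarts the ghost with them, then destroys that temporary actor.
; Spawning and killing the ghost toggle the controller's build-mode flag and a Tick gate that drives the snapped movement.
; Actual placement is absent here.
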(event `OnSpawn`
  (params (BuildingClass :type "/Game/Blueprints/Buildings/BP_Test_TycoonBaseBuilding Class Reference") (DisplayMesh :type "StaticMesh Object Reference") (ConstructionProxy :type "/Game/Blueprints/Construction/BP_ConstrtuctionProxy Class Reference"))
  ;[1 1 1] On spawn ghost
  (if (not (`self.IsActive`))
    (set `self.DisplayMesh` DisplayMesh)
    (set `self.BuildingClass` BuildingClass)
    (set `self.ConstructionProxy` ConstructionProxy)
    (set `self.IsActive` true)
    (set `/Game/Blueprints/Camera/BP_Test_TycoonCameraController.BuildModeActive` true (`self.ControllerRef`))
    (`StaticMeshComponent.SetStaticMesh` (`self.BaseMeshComponent`) (`self.DisplayMesh`))
    (`self.OpenTickGate`)))

(event `KillGhost`
  ;[1 1 1] Kill ghost
  (set `self.BuildingClass` null)
  (set `self.ConstructionProxy` null)
  (`self.CloseTickGate`)
  (set `self.DisplayMesh` null)
  (set `self.IsActive` false)
  (set `/Game/Blueprints/Camera/BP_Test_TycoonCameraController.BuildModeActive` false (`self.ControllerRef`)))

(event `/Game/Interfaces/I_HUD.ConstructBuilding`
  (params (BaseBuilding :type "/Game/Blueprints/Buildings/BP_Test_TycoonBaseBuilding Class Reference"))
  (bind _returnvalue (`|SpawnActorFromClass` BaseBuilding (`KismetMathLibrary.MakeTransform` (0.0 0.0 0.0)) "Undefined" "OverrideRootScale" null (`self.ControllerRef`) null))
  (`|ExecutionSequence`
    (:`then_0`
      (bind _asbp_test_tycoon_base_building (castclass `/Game/Blueprints/Buildings/BP_Test_TycoonBaseBuilding` BaseBuilding))
      (`self.KillGhost`)
      (`self.OnSpawn` _asbp_test_tycoon_base_building (`/Game/Blueprints/Buildings/BP_Test_TycoonBaseBuilding.DisplayMesh` _returnvalue) (`/Game/Blueprints/Buildings/BP_Test_TycoonBaseBuilding.ConstructionProxy` _returnvalue)))
    (:`then_1`
      (`self.K2_DestroyActor` _returnvalue))))

(event `self.ReceiveTick`
  (params (DeltaSeconds :type "Float (single-precision)"))
  (`/Engine/EditorBlueprintResources/StandardMacros.Gate` false :!label _label
    (:`Exit`
      (`self.K2_SetActorLocation` self (`self.SetGridSnapVector`) false false))))

(event `OpenTickGate`
  (goto _label :!via `Open`))

(event `CloseTickGate`
  (goto _label :!via `Close`))

(fn `SetCalendar`
  (params (Date :type "Array of Integer (by ref)"))
  (returns (Success :type Boolean))
  (return false))

(fn `SetClock`
  (params (Time :type "Array of Integer (by ref)"))
  (returns (Success :type Boolean))
  (return false))

(fn `SetGridSnapVector`
  (returns (GridSnap :type "Vector Structure"))
  (bind (_cursorworldposition_x _cursorworldposition_y _cursorworldposition_z) (`KismetMathLibrary.BreakVector` (`self.CursorWorldPosition`)))
  (bind _gridsize (`self.GridSize`))
  (return (`KismetMathLibrary.MakeVector` (`/Game/Blueprints/Libraries/Test_TycoonFunctionLibrary.GridSnap` _cursorworldposition_x _gridsize) (`/Game/Blueprints/Libraries/Test_TycoonFunctionLibrary.GridSnap` _cursorworldposition_y _gridsize) (`/Game/Blueprints/Libraries/Test_TycoonFunctionLibrary.GridSnap` _cursorworldposition_z _gridsize))))

(fn `UserConstructionScript`)