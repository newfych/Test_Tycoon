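; Placement ghost for build mode that previews a building's mesh at the cursor, snapped to a ground-level grid.
; ConstructBuilding briefly spawns the building class to read its mesh, proxy and work hours, then restarts the ghost with them.
; A gated Tick moves the ghost and swaps to an error material when it overlaps actors.
; GetConstructionStruct packages the placement transform and building data; KillGhost clears the preview and exits build mode.
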(event `OnSpawn`
  (params (BuildingClass :type "/Game/Blueprints/BuildingsClasses/BP_Test_TycoonBaseBuilding Class Reference") (DisplayMesh :type "StaticMesh Object Reference") (ConstructionProxy :type "/Game/Blueprints/Construction/BP_ConstrtuctionProxy Class Reference") (WorkHours :type "Float (double-precision)"))
  ;[1 1 1] On spawn ghost
  (if (not (`self.IsActive`))
    (set `self.DisplayMesh` DisplayMesh)
    (set `self.BuildingClass` BuildingClass)
    (set `self.ConstructionProxy` ConstructionProxy)
    (set `self.WorkHorsRequired` WorkHours)
    (set `self.IsActive` true)
    (set `/Game/Blueprints/Camera/BP_Test_TycoonCameraController.BuildModeActive` true (`self.ControllerRef`))
    (`StaticMeshComponent.SetStaticMesh` (`self.BaseMeshComponent`) (`self.DisplayMesh`))
    (`self.OpenTickGate`)
    (`self.SetMaterial` (not (`self.IsOverlapping`)))
    (set `self.Extent` (`.BoxExtent` (`KismetSystemLibrary.GetComponentBounds` (`self.BaseMeshComponent`))))))

(event `KillGhost`
  ;[1 1 1] Kill ghost
  (set `self.BuildingClass` null)
  (set `self.ConstructionProxy` null)
  (`self.CloseTickGate`)
  (set `self.DisplayMesh` null)
  (set `self.IsActive` false)
  (set `/Game/Blueprints/Camera/BP_Test_TycoonCameraController.BuildModeActive` false (`self.ControllerRef`))
  (`StaticMeshComponent.SetStaticMesh` (`self.BaseMeshComponent`) (`self.DisplayMesh`))
  (`self.K2_SetActorRotation` (struct)))

(event `/Game/Interfaces/I_HUD.ConstructBuilding`
  (params (BaseBuilding :type "/Game/Blueprints/BuildingsClasses/BP_Test_TycoonBaseBuilding Class Reference"))
  ;[1 1 1] Construct building
  (bind _returnvalue (`|SpawnActorFromClass` BaseBuilding (`KismetMathLibrary.MakeTransform` (0.0 0.0 0.0)) "Undefined" "OverrideRootScale" null (`self.ControllerRef`) null))
  (`|ExecutionSequence`
    (:`then_0`
      (bind _asbp_test_tycoon_base_building (castclass `/Game/Blueprints/BuildingsClasses/BP_Test_TycoonBaseBuilding` BaseBuilding))
      (`self.KillGhost`)
      (`self.OnSpawn` _asbp_test_tycoon_base_building (`/Game/Blueprints/BuildingsClasses/BP_Test_TycoonBaseBuilding.DisplayMesh` _returnvalue) (`/Game/Blueprints/BuildingsClasses/BP_Test_TycoonBaseBuilding.ConstructionProxy` _returnvalue) (`/Game/Blueprints/BuildingsClasses/BP_Test_TycoonBaseBuilding.ConstructionTime` _returnvalue)))
    (:`then_1`
      (`self.K2_DestroyActor` _returnvalue))))

(event `self.ReceiveTick`
  (params (DeltaSeconds :type "Float (single-precision)"))
  ;[1 1 1] Tick
  (`/Engine/EditorBlueprintResources/StandardMacros.Gate` false :!label _label
    (:`Exit`
      (`self.K2_SetActorLocation` self (`self.SetGridSnapVector`) false false)
      (if (`self.CheckOverlap`)
        (`self.SetMaterial` true)
        (else
          (`self.SetMaterial` false))))))

(event `OpenTickGate`
  ;[1 1 1] Tick
  (goto _label :!via `Open`))

(event `CloseTickGate`
  ;[1 1 1] Tick
  (goto _label :!via `Close`))

(event `SetMaterial`
  (params (IsError :type Boolean))
  (bind _basemeshcomponent (`self.BaseMeshComponent`))
  ;[1 1 1] SetMaterial
  (if (not (== IsError (`self.IsOverlapping`)))
    (bind _output_get (set `self.IsOverlapping` IsError))
    (if _output_get
      (`PrimitiveComponent.SetMaterial` _basemeshcomponent 0 "/Game/Materials/MI_Ghost_Error.MI_Ghost_Error")
      (else
        (`PrimitiveComponent.SetMaterial` _basemeshcomponent 0 "/Game/Materials/MI_Ghost.MI_Ghost")))))

(fn `CheckOverlap`
  (returns (Overlaping :type Boolean))
  (return (> (`KismetArrayLibrary.Array_Length` (`self.GetOverlappingActors` "/Script/Engine.Actor")) 0)))

(fn `GetConstructionStruct`
  (returns (ConstructionStruct :type "/Game/Structs/ConstructionStruct Structure"))
  (return (make `/Game/Structs/ConstructionStruct` (`self.BuildingClass`) (`self.ConstructionProxy`) (`KismetMathLibrary.MakeTransform` (`self.K2_GetActorLocation`) (`self.K2_GetActorRotation`)) (`self.DisplayMesh`) (`self.WorkHorsRequired`))))

(fn `SetCalendar`
  (params (Date :type "Array of Integer (by ref)"))
  (returns (Success :type Boolean))
  (return false))

(fn `SetClock`
  (params (Time :type "Array of Integer (by ref)"))
  (returns (Success :type Boolean))
  (return false))

(fn `SetCursorPosition`
  (params (CursorLocation :type "Vector Structure"))
  (set `self.CursorWorldPosition` CursorLocation)
  (return))

(fn `SetGridSnapVector`
  (returns (GridSnap :type "Vector Structure"))
  (bind (_cursorworldposition_x _cursorworldposition_y) (`KismetMathLibrary.BreakVector` (`self.CursorWorldPosition`)))
  (bind _gridsize (`self.GridSize`))
  (return (`KismetMathLibrary.MakeVector` (`/Game/Blueprints/Libraries/Test_TycoonFunctionLibrary.GridSnap` _cursorworldposition_x _gridsize) (`/Game/Blueprints/Libraries/Test_TycoonFunctionLibrary.GridSnap` _cursorworldposition_y _gridsize) (`/Game/Blueprints/Libraries/Test_TycoonFunctionLibrary.GridSnap` 0.0 _gridsize))))

(fn `UserConstructionScript`)