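; BP_Carpenter_House is a carpenter house building that periodically earns money for the player once construction finishes.
; Tick fills a progress value at a constant rate and pushes it to the W_Status money bar on its widget component.
; When the bar is full, it adds BuildingRevenue through the first BP_CameraController found, hides the widget, then restarts the cycle after a TimeToRestart delay.
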(event `OnConstructionFinished`
  (set `self.ConstructionFinished` true)
  (set `self.TimerIsActive` true))

(event `self.ReceiveTick`
  (params (DeltaSeconds :type "Float (single-precision)"))
  (bind _barpercent (`self.BarPercent`))
  (if (and (`self.ConstructionFinished`) (`self.TimerIsActive`))
    (bind _output_get (set `self.BarPercent` (`KismetMathLibrary.FInterpTo_Constant` (`self.BarPercent`) 1.0 DeltaSeconds 0.1)))
    (if (<= _output_get 1.0)
      (bind _asw_status (cast `/Game/UI/W_Status` (`WidgetComponent.GetUserWidgetObject` (`self.Widget`))))
      (`/Game/UI/W_Status.SetMoneyBarPercent` _asw_status _barpercent)
      (if (== _barpercent 1.0)
        (bind _outactors (`GameplayStatics.GetAllActorsOfClass` "/Game/Blueprints/Camera/BP_CameraController.BP_CameraController_C"))
        (`/Game/Blueprints/Camera/BP_CameraController.AddMoney` (`|GetArrayItem` _outactors) (`self.BuildingRevenue`))
        (`Widget.SetVisibility` (`WidgetComponent.GetUserWidgetObject` (`self.Widget`)) "Hidden")
        (set `self.TimerIsActive` false)
        (`KismetSystemLibrary.Delay` (`self.TimeToRestart`))
        (set `self.BarPercent` 0.0)
        (set `self.TimerIsActive` true)
        (`Widget.SetVisibility` (`WidgetComponent.GetUserWidgetObject` (`self.Widget`)) "Visible")))))

(fn `UserConstructionScript`
  (`parent.UserConstructionScript`))