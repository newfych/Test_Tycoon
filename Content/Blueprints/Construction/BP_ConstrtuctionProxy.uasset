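; Construction proxy actor for a tycoon game that shows a ghost-material mesh as a placeholder while a timed build runs.
; Tick advances a clockwork counter using the game state's time unit, refreshed through its game speed event, and debug-prints the remaining time.
; Once work time reaches the construction time set from work hours, it fires ConstructionCompleted with itself and destroys itself after a short delay.
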(event `self.ReceiveBeginPlay`
  ;[1 1 1] Begin Play
  (bind _output_get (set `self.GameStateRef` (cast `/Game/Blueprints/Base_Blueprints/BP_Test_TycoonGameState` (`GameplayStatics.GetGameState`) :!pure true)))
  (add `/Game/Blueprints/Base_Blueprints/BP_Test_TycoonGameState.UpdateGameSpeed` _output_get (`|CreateDelegate` :!event `AdjustTime`))
  (set `self.TimeUnit` (`/Game/Blueprints/Base_Blueprints/BP_Test_TycoonGameState.GetTimeUnit` (`self.GameStateRef`))))

(event `self.ReceiveTick`
  (params (DeltaSeconds :type "Float (single-precision)"))
  ;[1 1 1] Tick
  (set `self.Delta` DeltaSeconds)
  (if (not (`self.IsConstructionCompleted`))
    (`self.DoWork`)
    (if (>= (`self.WorkTimeSpent`) (`self.ConstructionTime`))
      (set `self.IsConstructionCompleted` true)
      (`self.ConstructionCompleted` self)
      (`KismetSystemLibrary.Delay` 0.2)
      (`self.K2_DestroyActor`))))

(event `AdjustTime`
  (params (TimeUnit :type "Float (double-precision)"))
  (set `self.TimeUnit` (`/Game/Blueprints/Base_Blueprints/BP_Test_TycoonGameState.GetTimeUnit` (`self.GameStateRef`))))

(fn `DoWork`
  (bind _output_get (set `self.Clockwork` (`/Game/Blueprints/Libraries/Test_TycoonFunctionLibrary.SetClockwork` (`self.Delta`) (`self.TimeUnit`) (`self.Clockwork`))))
  (bind _output_get_2 (set `self.WorkTimeSpent` (* _output_get 60.0)))
  (`KismetSystemLibrary.PrintString` (`KismetStringLibrary.Conv_DoubleToString` (- (`self.ConstructionTime`) _output_get_2)))
  (return))

(fn `SetConstructionTime`
  (params (WorkHours :type "Float (double-precision)"))
  (set `self.ConstructionTime` (* WorkHours 60.0))
  (return))

(fn `UserConstructionScript`
  (bind _staticmesh (`self.StaticMesh`))
  (`StaticMeshComponent.SetStaticMesh` _staticmesh (`self.DisplayMesh`))
  (`PrimitiveComponent.SetMaterial` _staticmesh 0 "/Game/Materials/MI_Ghost.MI_Ghost"))