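; Test function library of tycoon-game helpers for cursor placement, grid snapping and a 24-hour game clock.
; SetCursorWorldPosition deprojects the mouse and line-traces out to a sight distance, returning the location of an actor hit.
; GridSnap rounds a single axis value to the nearest grid multiple.
; SetClockwork adds scaled delta time to the clock, wraps it at 24 and outputs whole-day rollovers as DayTick.
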(fn `GridSnap`
  (params (Axis :type "Float (double-precision)") (GridSize :type Integer))
  (returns (AxisOut :type "Float (double-precision)"))
  (return (`KismetMathLibrary.Conv_IntToDouble` (* (`KismetMathLibrary.FFloor` (/ (+ Axis (`KismetMathLibrary.Conv_IntToDouble` (/ GridSize 2))) (`KismetMathLibrary.Conv_IntToDouble` GridSize))) GridSize))))

(fn `SetClockwork`
  (params (DeltaSeconds :type "Float (double-precision)") (TimeUnit :type "Float (double-precision)") (ClockworkIn :type "Float (double-precision)"))
  (returns (ClockworkOut :type "Float (double-precision)") (DayTick :type Integer))
  (bind (_remainder _returnvalue) (`KismetMathLibrary.FMod` (+ (/ DeltaSeconds TimeUnit) ClockworkIn) 24.0))
  (return _remainder _returnvalue))

(fn `SetCursorWorldPosition`
  (params (Controller :type "Test_TycoonPlayerController Object Reference") (SightDistance :type "Float (double-precision)"))
  (returns (Location :type "Vector Structure"))
  (bind (_worldlocation _worlddirection) (`PlayerController.DeprojectMousePositionToWorld` Controller))
  (bind _outhit (`KismetSystemLibrary.LineTraceSingle` null _worldlocation (+ _worldlocation (* _worlddirection SightDistance)) "TraceTypeQuery3"))
  (bind (_bblockinghit _binitialoverlap _time _distance _location _impactpoint _normal _impactnormal _physmat _hitactor) (`GameplayStatics.BreakHitResult` _outhit))
  (if (!= _hitactor null)
    (return _location)))