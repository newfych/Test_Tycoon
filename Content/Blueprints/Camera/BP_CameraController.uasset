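; Player controller for a tycoon builder that drives the camera pawn and handles building placement.
; On BeginPlay it spawns the construction manager, ghost building and economy manager, then creates the main HUD.
; Input handles zoom-scaled movement, screen-edge scrolling, gated mouse rotation and spring-arm zoom.
; In build mode, Tick moves the ghost to the cursor, keys rotate it, left-click queues valid placements and Deselect cancels with a refund.
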(event `self.ReceiveBeginPlay`
  (bind _returnvalue (`KismetMathLibrary.MakeTransform` (0.0 0.0 0.0)))
  ;[1 1 1] Begin Play
  (`|ExecutionSequence`
    (:`then_0`
      (`self.ReferenceCasts`))
    (:`then_1`
      (bind _returnvalue_2 (`|SpawnActorFromClass` "/Game/Blueprints/Construction/BP_ConstructionManager.BP_ConstructionManager_C" _returnvalue "AlwaysSpawn" "OverrideRootScale" null null))
      (set `self.ConstructionManagerRef` _returnvalue_2))
    (:`then_2`
      (bind _returnvalue_3 (`|SpawnActorFromClass` "/Game/Blueprints/BuildingsClasses/BP_GhostBuilding.BP_GhostBuilding_C" _returnvalue "Undefined" "OverrideRootScale" null self null))
      (set `self.GhostBuildingRef` _returnvalue_3))
    (:`then_3`
      (bind _returnvalue_4 (`|SpawnActorFromClass` "/Game/Blueprints/Economy/BP_EconomyManager.BP_EconomyManager_C" _returnvalue "Undefined" "OverrideRootScale" null 100 null))
      (set `self.EconomyManagerRef` _returnvalue_4))
    (:`then_4`
      (`WidgetBlueprintLibrary.SetInputMode_GameAndUIEx` self null "DoNotLock" false)
      (`self.CreateHUDs`)
      (`UserWidget.AddToViewport` (`self.MainHudRef`) 0))))

(event `InputAxis|MoveForward`
  (params (AxisValue :type "Float (single-precision)"))
  ;[1 1 1] X Axis movement
  (if (not (`self.DisableCamNav`))
    (`self.K2_SetActorTransform` (`self.CameraPawnRef`) (`self.MovementX` AxisValue (`self.MovementSpeedCalculation`) (`self.FastMoveMultiplier`) (`self.CameraPawnRef`)) false false)))

(event `InputAxis|MoveRight`
  (params (AxisValue :type "Float (single-precision)"))
  ;[1 1 1] Y Axis movement
  (if (not (`self.DisableCamNav`))
    (`self.K2_SetActorTransform` (`self.CameraPawnRef`) (`KismetMathLibrary.MakeTransform` (`KismetMathLibrary.MakeVector` (.x (.location (`self.MovementY` AxisValue (`self.MovementSpeedCalculation`) (`self.FastMoveMultiplier`) (`self.CameraPawnRef`)))) (.y (.location (`self.MovementY` AxisValue (`self.MovementSpeedCalculation`) (`self.FastMoveMultiplier`) (`self.CameraPawnRef`)))) 100.0) (.rotation (`self.MovementY` AxisValue (`self.MovementSpeedCalculation`) (`self.FastMoveMultiplier`) (`self.CameraPawnRef`))) (.scale (`self.MovementY` AxisValue (`self.MovementSpeedCalculation`) (`self.FastMoveMultiplier`) (`self.CameraPawnRef`)))) false false)))

(event `InputAction|PanReset`
  (params (Key :type "Key Structure"))
  ;[1 1 1] Pan Reset
  (:`Pressed`
    (`self.K2_SetActorRotation` (`self.CameraPawnRef`) (`KismetMathLibrary.MakeRotator` (.roll (`self.K2_GetActorRotation` (`self.CameraPawnRef`))) (.pitch (`self.K2_GetActorRotation` (`self.CameraPawnRef`)))) false)))

(event `InputAxisKey|MouseX`
  (params (AxisValue :type "Float (single-precision)"))
  ;[1 1 1] Pan X Axis
  (`/Engine/EditorBlueprintResources/StandardMacros.Gate` true :!label _label
    (:`Exit`
      (`self.K2_SetActorRotation` (`self.CameraPawnRef`) (`KismetMathLibrary.MakeRotator` (.roll (`self.K2_GetActorRotation` (`self.CameraPawnRef`))) (.pitch (`self.K2_GetActorRotation` (`self.CameraPawnRef`))) (+ (.yaw (`self.K2_GetActorRotation` (`self.CameraPawnRef`))) (* (`self.PanSensitivity`) AxisValue))) false))))

(event `InputAction|Pan`
  (params (Key :type "Key Structure"))
  ;[1 1 1] Pan X Axis
  (:`Pressed`
    (set `self.DisableCamNav` true)
    (goto _label :!via `Open`))
  (:`Released`
    (set `self.DisableCamNav` false)
    (goto _label :!via `Close`)))

(event `Key|LeftShift`
  (params (Key :type "Key Structure"))
  ;[1 1 1] Set Move Multiplier
  (:`Pressed`
    (set `self.FastMoveMultiplier` 2.0))
  (:`Released`
    (set `self.FastMoveMultiplier` 1.0)))

(event `InputAxisKey|MouseY`
  (params (AxisValue :type "Float (single-precision)"))
  ;[1 1 1] Pan Y Axis
  (`/Engine/EditorBlueprintResources/StandardMacros.Gate` true :!label _label_2
    (:`Exit`
      (`self.K2_SetActorRotation` (`self.CameraPawnRef`) (`KismetMathLibrary.MakeRotator` (.roll (`self.K2_GetActorRotation` (`self.CameraPawnRef`))) (`KismetMathLibrary.FClamp` (+ (.pitch (`self.K2_GetActorRotation` (`self.CameraPawnRef`))) (* (`self.PanSensitivity`) AxisValue)) -15.0 50.0) (.yaw (`self.K2_GetActorRotation` (`self.CameraPawnRef`)))) false))))

(event `InputAction|Pan`
  (params (Key :type "Key Structure"))
  ;[1 1 1] Pan Y Axis
  (:`Pressed`
    (set `self.DisableCamNav` true)
    (goto _label_2 :!via `Open`))
  (:`Released`
    (set `self.DisableCamNav` false)
    (goto _label_2 :!via `Close`)))

(event `InputAxisKey|MouseX`
  (params (AxisValue :type "Float (single-precision)"))
  ;[1 1 1] Camera Edge movement
  (if (not (`self.DisableCamNav`))
    (`|ExecutionSequence` :!label _label_3
      (:`then_0`
        (bind (_deltaxspeed _deltayspeed) (`self.ScreenEdgeMovements` :!label _label_4))
        (`self.K2_AddActorLocalOffset` (`self.CameraPawnRef`) (`KismetMathLibrary.MakeVector` _deltaxspeed _deltayspeed) true false))
      (:`then_1`
        (goto _label_4 :!via `MouseY`)))))

(event `InputAction|Zoom in`
  (params (Key :type "Key Structure"))
  (bind _springarm (`/Game/Blueprints/Camera/BP_CameraPawn.SpringArm` (`self.CameraPawnRef`)))
  ;[1 1 1] Zoom in/out
  (:`Pressed`
    (set `SpringArmComponent.TargetArmLength` (`KismetMathLibrary.FClamp` (/ (`SpringArmComponent.TargetArmLength` _springarm) (`self.ZoomSpeed`)) 800.0 (`self.MaxCameraArmLength`)) _springarm)))

(event `InputAxisKey|MouseY`
  (params (AxisValue :type "Float (single-precision)"))
  ;[1 1 1] Camera Edge movement
  (if (not true)
    (goto _label_3)))

(event `InputAction|Zoom out`
  (params (Key :type "Key Structure"))
  (bind _springarm (`/Game/Blueprints/Camera/BP_CameraPawn.SpringArm` (`self.CameraPawnRef`)))
  ;[1 1 1] Zoom in/out
  (:`Pressed`
    (set `SpringArmComponent.TargetArmLength` (`KismetMathLibrary.FClamp` (* (`SpringArmComponent.TargetArmLength` _springarm) (`self.ZoomSpeed`)) 800.0 (`self.MaxCameraArmLength`)) _springarm)))

(event `InputAction|ZoomReset`
  (params (Key :type "Key Structure"))
  ;[1 1 1] Zoom reset
  (:`Pressed`
    (set `SpringArmComponent.TargetArmLength` 1500.0 (`/Game/Blueprints/Camera/BP_CameraPawn.SpringArm` (`self.CameraPawnRef`)))))

(event `self.ReceiveTick`
  (params (DeltaSeconds :type "Float (single-precision)"))
  ;[1 1 1] Tick
  (if (`self.BuildModeActive`)
    (if (!= (`self.GhostBuildingRef`) null)
      (`/Game/Blueprints/BuildingsClasses/BP_GhostBuilding.SetCursorPosition` (`self.GhostBuildingRef`) (`/Game/Blueprints/Libraries/Test_TycoonFunctionLibrary.SetCursorWorldPosition` self (`self.SetSightDistance`))))))

(event `InputAction|Deselect`
  (params (Key :type "Key Structure"))
  ;[1 1 1] Deselect
  (:`Pressed`
    (if (`self.BuildModeActive`)
      (`/Game/Blueprints/BuildingsClasses/BP_GhostBuilding.KillGhost` (`self.GhostBuildingRef`))
      (set `self.BuildModeActive` false)
      (`/Game/Blueprints/Economy/BP_EconomyManager.AddMoney` (`self.EconomyManagerRef`) (`self.MoneyOnUndo`))
      (set `self.MoneyOnUndo` 0)
      (`/Game/UI/W_MainHUD.Set Money AmountText` (`self.MainHudRef`)))))

(event `Key|LeftMouseButton`
  (params (Key :type "Key Structure"))
  (bind _ghostbuildingref (`self.GhostBuildingRef`))
  ;[1 1 1] Left mouse click
  (:`Pressed`
    (if (and (`self.BuildModeActive`) (not (`/Game/Blueprints/BuildingsClasses/BP_GhostBuilding.IsOverlapping` _ghostbuildingref)) (!= _ghostbuildingref null))
      (bind _constructionstruct (`/Game/Blueprints/BuildingsClasses/BP_GhostBuilding.GetConstructionStruct` (`self.GhostBuildingRef`)))
      (`/Game/Blueprints/Construction/BP_ConstructionManager.QueueConstruction` (`self.ConstructionManagerRef`) _constructionstruct)
      (`/Game/Blueprints/BuildingsClasses/BP_GhostBuilding.KillGhost` (`self.GhostBuildingRef`)))))

(event `InputAction|RotateBuildingRight`
  (params (Key :type "Key Structure"))
  (bind _ghostbuildingref (`self.GhostBuildingRef`))
  ;[1 1 1] Left mouse click
  ;;[1 1 1] Building Rotation
  (:`Pressed`
    (if (and (`KismetSystemLibrary.IsValid` _ghostbuildingref) (`self.BuildModeActive`))
      (`self.K2_SetActorRotation` _ghostbuildingref (`KismetMathLibrary.MakeRotator` (.roll (`self.K2_GetActorRotation` _ghostbuildingref)) (.pitch (`self.K2_GetActorRotation` _ghostbuildingref)) (- (.yaw (`self.K2_GetActorRotation` _ghostbuildingref)) (`self.BuildingRotationRate`))) false))))

(event `InputAction|RotateBuildingLeft`
  (params (Key :type "Key Structure"))
  (bind _ghostbuildingref (`self.GhostBuildingRef`))
  ;[1 1 1] Left mouse click
  ;;[1 1 1] Building Rotation
  (:`Pressed`
    (if (and (`KismetSystemLibrary.IsValid` _ghostbuildingref) (`self.BuildModeActive`))
      (`self.K2_SetActorRotation` _ghostbuildingref (`KismetMathLibrary.MakeRotator` (.roll (`self.K2_GetActorRotation` _ghostbuildingref)) (.pitch (`self.K2_GetActorRotation` _ghostbuildingref)) (+ (.yaw (`self.K2_GetActorRotation` _ghostbuildingref)) (`self.BuildingRotationRate`))) false))))

(event `InputAction|ShowHideHelp`
  (params (Key :type "Key Structure"))
  ;[1 1 1] Show/hide help
  (:`Pressed`
    (bind _isa (`/Engine/EditorBlueprintResources/StandardMacros.FlipFlop`)
      (:`A`
        (set `self.HelpVisible` false))
      (:`B`
        (set `self.HelpVisible` true)))
    (message `/Game/Interfaces/I_HUD.ShowHelp` (`self.MainHudRef`) _isa)))

(event `AddMoney`
  (params (MoneyAmount :type Integer)))

(fn `MovementSpeedCalculation`
  (returns (MoveSensitivity :type "Float (double-precision)"))
  (return (`KismetMathLibrary.FClamp` (/ (`SpringArmComponent.TargetArmLength` (`/Game/Blueprints/Camera/BP_CameraPawn.SpringArm` (`self.CameraPawnRef`))) (`self.CameraMoveMultiplier`)) (`self.MinCameraSpeed`) (`self.MaxCameraSpeed`))))

(fn `SetBackMoneyOnUndo`
  (params (MoneyAmount :type Integer))
  (`/Game/Blueprints/Economy/BP_EconomyManager.AddMoney` (`self.EconomyManagerRef`) MoneyAmount))

(fn `SetCalendar`
  (params (Date :type "Array of Integer (by ref)"))
  (returns (Success :type Boolean))
  (return false))

(fn `SetClock`
  (params (Time :type "Array of Integer (by ref)"))
  (returns (Success :type Boolean))
  (return false))

(fn `SetSightDistance`
  (returns (SightDistance :type "Float (double-precision)"))
  (return (+ (`SpringArmComponent.TargetArmLength` (`/Game/Blueprints/Camera/BP_CameraPawn.SpringArm` (`self.CameraPawnRef`))) (`self.SightDistance`))))

(fn `UserConstructionScript`)